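; Left leg body-part pickup actor that the player can collect once.
; Overlapping its Box while the part is present shows a prompt Widget and sets TapKeyVisibility; leaving hides both.
; The getBody event, with no caller in this graph, checks both flags, waits through a Delay, then hides the Body and clears HasBody.
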(event `self.ReceiveBeginPlay`
  (set `self.hasBody` true))

(event `self.Box.OnComponentBeginOverlap`
  (params (OverlappedComponent :type "PrimitiveComponent Object Reference") (OtherActor :type "Actor Object Reference") (OtherComp :type "PrimitiveComponent Object Reference") (OtherBodyIndex :type Integer) (bFromSweep :type Boolean) (SweepResult :type "HitResult Structure (by ref)"))
  ;[1 1 1] 박스 위 ui
  (if (`self.hasBody`)
    (`SceneComponent.SetVisibility` (`self.Widget`) true false)
    (set `self.TapKeyVisibility` true)))

(event `self.Box.OnComponentEndOverlap`
  (params (OverlappedComponent :type "PrimitiveComponent Object Reference") (OtherActor :type "Actor Object Reference") (OtherComp :type "PrimitiveComponent Object Reference") (OtherBodyIndex :type Integer))
  ;[1 1 1] 박스 위 ui
  (`SceneComponent.SetVisibility` (`self.Widget`) false false)
  (set `self.TapKeyVisibility` false))

(event `getBody`
  ;[1 1 1] 다리 획득
  (if (and (`self.TapKeyVisibility`) (`self.hasBody`))
    (`KismetSystemLibrary.Delay` 3.0)
    (`KismetSystemLibrary.PrintString` "Get Body")
    (`SceneComponent.SetVisibility` (`self.body`) false false)
    (set `self.hasBody` false)))

(fn `UserConstructionScript`)