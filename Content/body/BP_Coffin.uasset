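; BP_Coffin is a coffin actor that reveals leg parts according to the body count carried by BP_Yuri.
; Box overlap begin and end toggle a TapKeyVisibility flag, then run the same check that Tick runs every frame.
; That check casts the begin-overlap actor to BP_Yuri and switches on BodyCount to show the first, second or third leg.
; Widget visibility calls are present but never run.
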(event `self.ReceiveTick`
  (params (DeltaSeconds :type "Float (single-precision)"))
  (bind _asbp_yuri (cast `/Game/MetaHumans/Yuri/BP_Yuri` (stale `self.Box.OnComponentBeginOverlap` OtherActor) :!label _label))
  (switch `int` (`/Game/MetaHumans/Yuri/BP_Yuri.BodyCount` _asbp_yuri)
    (:`1`
      (`SceneComponent.SetVisibility` (`self.leg1`) true false))
    (:`2`
      (`SceneComponent.SetVisibility` (`self.leg2`) true false))
    (:`3`
      (`SceneComponent.SetVisibility` (`self.leg3`) true false))))

(event `self.Box.OnComponentBeginOverlap`
  (params (OverlappedComponent :type "PrimitiveComponent Object Reference") (OtherActor :type "Actor Object Reference") (OtherComp :type "PrimitiveComponent Object Reference") (OtherBodyIndex :type Integer) (bFromSweep :type Boolean) (SweepResult :type "HitResult Structure (by ref)"))
  (set `self.Tap Key Visibility` true)
  (goto _label))

(event `self.Box.OnComponentEndOverlap`
  (params (OverlappedComponent :type "PrimitiveComponent Object Reference") (OtherActor :type "Actor Object Reference") (OtherComp :type "PrimitiveComponent Object Reference") (OtherBodyIndex :type Integer))
  (set `self.Tap Key Visibility` false)
  (goto _label))

(fn `UserConstructionScript`)