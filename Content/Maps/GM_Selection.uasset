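; Game mode for the selection map that spawns a display character as players log in.
; PostLogin increments PlayerCount and switches on it, spawning the Ghost selection character for count 1 and the Yuri selection mesh for count 2 at fixed transforms.
; BeginPlay sets the count to 1.
; The server-to-multicast count events end in an empty handler, and the selection menu widget and input setup are disconnected.
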(event `self.ReceiveBeginPlay`
  (set `self.PlayerCount` 1))

(event `self.ReceiveTick`
  (params (DeltaSeconds :type "Float (single-precision)")))

(event `self.K2_PostLogin`
  (params (NewPlayer :type "PlayerController Object Reference"))
  (bind _playercount (`self.PlayerCount`))
  (set `self.PlayerCount` (+ (`self.PlayerCount`) 1))
  (switch `int` (`self.PlayerCount`)
    (:`1`
      (bind _output_get (set `self.Spawn Transform` (`KismetMathLibrary.MakeTransform` (327.0 -337.0 142.0) (struct :`Yaw` 180.0))))
      (`|SpawnActorFromClass` "/Game/Maps/ghost_character_Selection.ghost_character_Selection_C" _output_get "Undefined" "MultiplyWithRoot" null null)
      (`KismetSystemLibrary.PrintString` (`KismetStringLibrary.Conv_IntToString` _playercount)))
    (:`2`
      (bind _output_get_2 (set `self.Spawn Transform` (`KismetMathLibrary.MakeTransform` (327.331 -85.0 124.0) (struct :`Yaw` 180.0))))
      (`|SpawnActorFromClass` "/Game/Maps/BP_Yuri_onlySM_selection.BP_Yuri_onlySM_selection_C" _output_get_2 "Undefined" "MultiplyWithRoot" null null)
      (`KismetSystemLibrary.PrintString` (`KismetStringLibrary.Conv_IntToString` _playercount)))))

(event `Server PlayerCount`
  (params (PlayerCount :type Integer))
  (`self.MulticastPlayertCount` PlayerCount))

(event `MulticastPlayertCount`
  (params (PlayerCount :type Integer)))

(fn `UserConstructionScript`)