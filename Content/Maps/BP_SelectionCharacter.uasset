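; BP_SelectionCharacter is a Blueprint that previews selectable characters on a skeletal mesh, apparently for a character selection screen.
; Its ChangeCharacter event advances an index through the Characters array, wrapping back to the first entry after the last.
; It then assigns the skeletal mesh asset at that index to the SkeletalMesh component.
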(event `Change Character`
  (if (< (`self.currentCharacterIndex`) (- (`KismetArrayLibrary.Array_Length` (`self.Characters`)) 1))
    (`/Engine/EditorBlueprintResources/StandardMacros.IncrementInt` (`self.currentCharacterIndex`)
      (:`  `
        _))
    (else
      (set `self.currentCharacterIndex` 0)))
  (`SkeletalMeshComponent.SetSkeletalMeshAsset` (`self.SkeletalMesh`) (`|GetArrayItem` (`self.Characters`) (`self.currentCharacterIndex`))))

(fn `UserConstructionScript`)